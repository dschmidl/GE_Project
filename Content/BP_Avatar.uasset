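; BP_Avatar is a player avatar controlled through Kinect body tracking.
; Each Tick it reads the centered body: ankle separation sets one of two forward speeds along the camera's facing, moving the capsule without sweep.
; A short head-to-ankle distance triggers Crouch, checked only while moving, with just a debug print in place of standing up.
; An open right hand triggers Jump, and a left-hand lasso calls OnFire.
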(event `self.ReceiveTick`
  (params (DeltaSeconds :type "Float (single-precision)"))
  ;[1 1 1] Vorwärts
  (bind _centeredbody (`KinectInterfaceComponent.GetCenteredBody` (`self.KinectInterface`)))
  (`|ExecutionSequence`
    (:`then_0`
      (bind _returnvalue (`KinectInterfaceComponent.GetDistanceBetweenJoints` (`self.KinectInterface`) "AnkleLeft" "AnkleRight" _centeredbody))
      (`/Engine/EditorBlueprintResources/StandardMacros.CompareFloat` _returnvalue 65.0
        (:`>`
          (`SceneComponent.K2_AddWorldOffset` (`self.CapsuleComponent`) (* (`KismetMathLibrary.Conv_RotatorToVector` (`SceneComponent.K2_GetComponentRotation` (`self.Camera`))) 5) false false))
        (:`<`
          (`/Engine/EditorBlueprintResources/StandardMacros.CompareFloat` _returnvalue 35.0
            (:`>`
              (`SceneComponent.K2_AddWorldOffset` (`self.CapsuleComponent`) (* (`KismetMathLibrary.Conv_RotatorToVector` (`SceneComponent.K2_GetComponentRotation` (`self.Camera`))) 2) false false)))))
      ;[1 1 1] Ducken
      (bind _returnvalue_2 (`KinectInterfaceComponent.GetDistanceBetweenJoints` (`self.KinectInterface`) "Head" "AnkleRight" _centeredbody))
      (`/Engine/EditorBlueprintResources/StandardMacros.CompareFloat` _returnvalue_2 110.0
        (:`>`
          ;;[1 1 1] Avatar muss wieder gerade stehen
          (`KismetSystemLibrary.PrintString` "Hello"))
        (:`<`
          (`self.Crouch`))))
    (:`then_1`
      ;[1 1 1] Springen
      (`KinectInterfaceComponent.GetHandStateAsExecution` (`self.KinectInterface`) "Right" _centeredbody
        (:`Open`
          (`KismetSystemLibrary.PrintString` "jeeeeeeeeeeeeeeeeeeeeeeeeeeeeeeeeee")
          (`self.Jump`))))
    (:`then_2`
      (`KinectInterfaceComponent.GetHandStateAsExecution` (`self.KinectInterface`) "Left" _centeredbody
        (:`Lasso`
          (`KismetSystemLibrary.PrintString` "schuss")
          (`self.OnFire`))))))

(fn `UserConstructionScript`)