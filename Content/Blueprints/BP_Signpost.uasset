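; BP_Signpost is a signpost with up to six text lines and a configurable text colour, set up in its construction script.
; A sequence destroys the text render component of each empty string: Title, Description and Line3 to Line6.
; Only Title is written to its component here; the other strings are just checked for length.
; The colour is then applied to the first five text components, leaving the sixth unchanged.
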(fn `UserConstructionScript`
  (bind _title (`self.Title`))
  (`|ExecutionSequence`
    (:`then_0`
      (if (== (`KismetStringLibrary.Len` _title) 0)
        (`ActorComponent.K2_DestroyComponent` (`self.TextRender1`))
        (else
          (`TextRenderComponent.K2_SetText` (`self.TextRender1`) (`KismetTextLibrary.Conv_StringToText` _title)))))
    (:`then_1`
      (if (== (`KismetStringLibrary.Len` (`self.Description`)) 0)
        (`ActorComponent.K2_DestroyComponent` (`self.TextRender2`))))
    (:`then_2`
      (if (== (`KismetStringLibrary.Len` (`self.Line3`)) 0)
        (`ActorComponent.K2_DestroyComponent` (`self.TextRender3`))))
    (:`then_3`
      (if (== (`KismetStringLibrary.Len` (`self.Line4`)) 0)
        (`ActorComponent.K2_DestroyComponent` (`self.TextRender4`))))
    (:`then_4`
      (if (== (`KismetStringLibrary.Len` (`self.Line5`)) 0)
        (`ActorComponent.K2_DestroyComponent` (`self.TextRender5`))))
    (:`then_5`
      (if (== (`KismetStringLibrary.Len` (`self.Line6`)) 0)
        (`ActorComponent.K2_DestroyComponent` (`self.TextRender6`))))
    (:`then_6`
      (`TextRenderComponent.SetTextRenderColor` (`self.TextRender1`) (`KismetMathLibrary.Conv_LinearColorToColor` (`self.TextColour`)))
      (`TextRenderComponent.SetTextRenderColor` (`self.TextRender2`) (`KismetMathLibrary.Conv_LinearColorToColor` (`self.TextColour`)))
      (`TextRenderComponent.SetTextRenderColor` (`self.TextRender3`) (`KismetMathLibrary.Conv_LinearColorToColor` (`self.TextColour`)))
      (`TextRenderComponent.SetTextRenderColor` (`self.TextRender4`) (`KismetMathLibrary.Conv_LinearColorToColor` (`self.TextColour`)))
      (`TextRenderComponent.SetTextRenderColor` (`self.TextRender5`) (`KismetMathLibrary.Conv_LinearColorToColor` (`self.TextColour`))))))